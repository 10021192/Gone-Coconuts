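; Player controller for GoneCoconuts that sets up the local player's HUD and game input.
; On BeginPlay, the local controller switches to game-only input, hides the cursor, and creates and displays W_PlayerHUD.
; The inventory input action opens the player menu through that HUD.
; EnableAllInput, GameStartCountdown and UIShowIngameHUD do nothing, as their input and WB_InGameHUD logic is disconnected.
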(event Custom|EnableAllInput)

(event Custom|GameStartCountdown)

(event Input|EnhancedActionEvents|EnhancedInputActionIA_Inventory
  (params (ActionValue :type Boolean) (ElapsedSeconds :type Float%20%28double-precision%29) (TriggeredSeconds :type Float%20%28double-precision%29) (InputAction :type Input%20Action%20Object%20Reference :default "/Game/FirstPerson/Input/Actions/IA_Inventory.IA_Inventory"))
  (:Triggered
    (Default|DisplayPlayerMenu (Variables|Default|GetHUD))))

(event EventBeginPlay
  (if (Pawn|IsLocalPlayerController)
    (Utilities|FlowControl|Sequence
      (:then_0
        (Input|SetInputModeGameOnly self false)
        (Variables|Default|SetbShowMouseCursor false))
      (:then_1
        (bind _returnvalue (UserInterface|CreateWidget "/Game/W_PlayerHUD.W_PlayerHUD_C"))
        (bind _output_get (Variables|Default|SetHUD _returnvalue))
        (UserInterface|Viewport|AddtoViewport _output_get 0)))))

(fn ConstructionScript)

(fn UIShowIngameHUD)