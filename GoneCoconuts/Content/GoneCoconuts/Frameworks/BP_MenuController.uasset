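; BP_MenuController is the player controller for the menus and multiplayer lobby, giving the local player a cursor and UI-only input.
; It loads the player profile from a save slot, creating one if missing, then passes it to the server, which has BP_MenuGamemode update the lobby.
; It also creates the lobby widget, refreshes its player names, and destroys the session before returning to the main menu map.
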(event Custom|EndClientSession
  (|DestroySession self
    (:then
      (Game|OpenLevel(byName) "MainMenu_Map"))))

(event Custom|CreateLobbyMenu
  (CallFunction|UIShowLobbyMenu))

(event Custom|InitialSetup
  (CallFunction|LoadSavedProfile)
  (CallFunction|ServerUpdateLobby (Variables|Default|GetPlayerProfileInfo)))

(event Custom|UpdatePlayerNames
  (params (Player%20Profiles :type Array%20of%20S%20Player%20Profile%20Structures))
  (bind _wb_lobbymenu (Variables|Default|GetWB_LobbyMenu))
  (Utilities|IsValid _wb_lobbymenu
    (:Is%20Valid
      (Default|ClearPlayerNames _wb_lobbymenu)
      (Default|UpdatePlayerNames _wb_lobbymenu Player%20Profiles))))

(event Custom|Server_UpdateLobby
  (params (Player%20Profile :type S%20Player%20Profile%20Structure))
  (Variables|Default|SetPlayerProfileInfo Player%20Profile)
  (bind _asbp_menu_gamemode (Utilities|Casting|CastToBP_MenuGamemode (Game|GetGameMode)))
  (Default|UpdateLobby _asbp_menu_gamemode true))

(event EventTick
  (params (DeltaSeconds :type Float%20%28single-precision%29)))

(event EventBeginPlay
  (if (Pawn|IsLocalController)
    (Variables|Default|SetbShowMouseCursor true)
    (Input|SetInputModeUIOnly self 0 "DoNotLock" false)))

(fn ConstructionScript)

(fn UIShowLobbyMenu
  (Utilities|IsValid (Variables|Default|GetWB_LobbyMenu)
    (:Is%20Valid
      _)
    (:Is%20Not%20Valid
      (bind _returnvalue (UserInterface|CreateWidget "/Game/GoneCoconuts/User_Interface/WB_LobbyMenu.WB_LobbyMenu_C" self))
      (Variables|Default|SetWB_LobbyMenu _returnvalue)))
  (UserInterface|Viewport|AddtoViewport (Variables|Default|GetWB_LobbyMenu) 0)
  (return))

(fn LoadSavedProfile
  (bind _returnvalue (SaveGame|DoesSaveGameExist (LocalVariables|GetLocal_Slot%20Name)))
  (if _returnvalue
    _
    (else
      (bind _returnvalue_2 (SaveGame|CreateSaveGameObject "/Game/GoneCoconuts/SavedData/SG_PlayerProfile.SG_PlayerProfile_C"))
      (SaveGame|SaveGametoSlot _returnvalue_2 (LocalVariables|GetLocal_Slot%20Name))))
  (bind _returnvalue_3 (SaveGame|LoadGamefromSlot (LocalVariables|GetLocal_Slot%20Name)))
  (bind _assg_player_profile (Utilities|Casting|CastToSG_PlayerProfile _returnvalue_3))
  (Variables|Default|SetPlayerProfileInfo (Variables|/Game/GoneCoconuts/SavedData/SG_PlayerProfile.SG_PlayerProfile_C|GetPlayerProfile _assg_player_profile))
  (return))